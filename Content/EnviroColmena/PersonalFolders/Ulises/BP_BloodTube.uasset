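; BP_BloodTube is a spline-based construction actor that builds a blood tube from repeated mesh segments along an editable path.
; The construction script takes segment length from a tube mesh's Y bounds, then adds Y-forward spline mesh components with collision along the spline.
; Each segment randomly picks Tube1 or Tube2, with tangents clamped to segment length.
; Tube3 is unused, and the event graph has no active logic.
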(event EventBeginPlay)

(event Collision|EventActorBeginOverlap
  (params (OtherActor :type Actor%20Object%20Reference)))

(event EventTick
  (params (DeltaSeconds :type Float%20%28single-precision%29)))

(fn ConstructionScript
  (bind _tube1 (Variables|Default|GetTube1))
  (bind _tube2 (Variables|Default|GetTube2))
  (bind _spline (Variables|Default|GetSpline))
  (bind _spline_2 (Variables|Default|GetSpline))
  (bind _array (Utilities|Array|MakeArray _tube1 _tube2))
  (bind _returnvalue (Utilities|Array|LastIndex _array))
  (bind _returnvalue_2 (Math|Random|RandomIntegerinRange 0 _returnvalue))
  (bind _output (Utilities|Array|Get(acopy) _array _returnvalue_2))
  (bind _returnvalue_3 (StaticMesh|GetBoundingBox _output))
  (bind _output_get (Variables|Default|SetYLenght (.y (+ (Math|Vector|VectorGetAbs (.min _returnvalue_3)) (Math|Vector|VectorGetAbs (.max _returnvalue_3))))))
  (for _index (range 0 (Math|Float|Truncate (/ (Spline|GetSplineLength (Variables|Default|GetSpline)) _output_get)))
    (bind _returnvalue_4 (AddComponent|AddSplineMeshComponent false))
    (Collision|SetCollisionEnabled _returnvalue_4 "QueryAndPhysics")
    (SplineMesh|SetForwardAxis _returnvalue_4 "Y" true)
    (Components|StaticMesh|SetStaticMesh _returnvalue_4 _output)
    (SplineMesh|SetStartandEnd _returnvalue_4 (Spline|GetLocationatDistanceAlongSpline _spline_2 (* _index (Variables|Default|GetYLenght)) "Local") (Math|Vector|ClampVectorSize (Spline|GetTangentatDistanceAlongSpline _spline_2 (* _index (Variables|Default|GetYLenght)) "Local") 0.0 (Variables|Default|GetYLenght)) (Spline|GetLocationatDistanceAlongSpline _spline (* (+ _index 1) (Variables|Default|GetYLenght)) "Local") (Math|Vector|ClampVectorSize (Spline|GetTangentatDistanceAlongSpline _spline (* (+ _index 1) (Variables|Default|GetYLenght)) "Local") 0.0 (Variables|Default|GetYLenght)) true :!class /Script/Engine.SplineMeshComponent)))